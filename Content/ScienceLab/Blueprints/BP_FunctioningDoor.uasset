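; BP_FunctioningDoor is a science lab sliding double door that opens and closes from overlaps on its Collision component.
; Begin overlap plays a timeline that slides the two panels apart in opposite directions along local Y.
; End overlap plays a second timeline whose output is multiplied by zero, so both panels snap to zero Y.
; The BP_Body casts on actor overlap events lead nowhere, so they do not filter the door triggers.
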(event OnComponentBeginOverlap(Collision)
  (params (OverlappedComponent :type Primitive%20Component%20Object%20Reference) (OtherActor :type Actor%20Object%20Reference) (OtherComp :type Primitive%20Component%20Object%20Reference) (OtherBodyIndex :type Integer) (bFromSweep :type Boolean) (SweepResult :type Hit%20Result%20Structure%20%28by%20ref%29))
  ;[0 0.3281 0] SecurityBreach0X00CF52
  (bind _open_door (Timeline|Timeline Play)
    (:Update
      (Transformation|SetRelativeLocation (Variables|Default|GetLabDoor03A) (Math|Vector|MakeVector 0.0 (* _open_door -1e+02) 0.0) false false)
      (Transformation|SetRelativeLocation (Variables|Default|GetLabDoor03B) (Math|Vector|MakeVector 0.0 (* (* _open_door -1e+02) -1.0) 0.0) false false))))

(event OnComponentEndOverlap(Collision)
  (params (OverlappedComponent :type Primitive%20Component%20Object%20Reference) (OtherActor :type Actor%20Object%20Reference) (OtherComp :type Primitive%20Component%20Object%20Reference) (OtherBodyIndex :type Integer))
  ;[0 0.3281 0] SecurityBreach0X00CF52
  (bind _close_door (Timeline|Timeline_0 Play)
    (:Update
      (Transformation|SetRelativeLocation (Variables|Default|GetLabDoor03A) (Math|Vector|MakeVector 0.0 (* _close_door 0.0) 0.0) false false)
      (Transformation|SetRelativeLocation (Variables|Default|GetLabDoor03B) (Math|Vector|MakeVector 0.0 (* _close_door 0.0) 0.0) false false))))

(event Collision|EventActorBeginOverlap
  (params (OtherActor :type Actor%20Object%20Reference))
  ;[0 0.3281 0] SecurityBreach0X00CF52
  (Utilities|Casting|CastToBP_Body OtherActor))

(event Collision|EventActorEndOverlap
  (params (OtherActor :type Actor%20Object%20Reference))
  ;[0 0.3281 0] SecurityBreach0X00CF52
  (Utilities|Casting|CastToBP_Body OtherActor))

(fn ConstructionScript)