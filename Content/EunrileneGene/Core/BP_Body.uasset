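; BP_Body is a first-person player character handling movement, look and interaction through Enhanced Input.
; On possession it adds the movement mapping context, then moves along camera yaw and feeds look input to player character 0.
; Interact runs a short, debug-drawn camera line trace and sends an interaction message to the hit component.
; Overlapping actors receive a hardcoded ID check message, and the construction script calls an obscurely named Add function.
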(event Input|EnhancedActionEvents|EnhancedInputActionIA_Look
  (params (ActionValue :type Vector%202D%20Structure) (ElapsedSeconds :type Float%20%28double-precision%29) (TriggeredSeconds :type Float%20%28double-precision%29) (InputAction :type Input%20Action%20Object%20Reference :default "/Game/EunrileneGene/Inputs/Action/IA_Look.IA_Look"))
  (bind _returnvalue (Game|GetPlayerCharacter 0))
  ;[0.006671 0.151 0] HeadRotation
  (:Triggered
    (Pawn|Input|AddControllerYawInput _returnvalue (.x ActionValue))
    (Pawn|Input|AddControllerPitchInput _returnvalue (.y ActionValue))))

(event Input|EnhancedActionEvents|EnhancedInputActionIA_Interact
  (params (ActionValue :type Boolean) (ElapsedSeconds :type Float%20%28double-precision%29) (TriggeredSeconds :type Float%20%28double-precision%29) (InputAction :type Input%20Action%20Object%20Reference :default "/Game/EunrileneGene/Inputs/Action/IA_Interact.IA_Interact"))
  (bind _firstpersoncamera (Variables|MyCharacter|GetFirstPersonCamera))
  (bind _returnvalue (Transformation|GetWorldLocation _firstpersoncamera))
  ;[0 0.3281 0] NeuralPsychicInteractionV2.0
  (:Started
    (bind _outhit (Collision|LineTraceByChannel _returnvalue (+ _returnvalue (* (Math|Vector|GetForwardVector _firstpersoncamera) 2e+02)) "TraceTypeQuery1" false 0 "ForDuration"))
    (Class|BPISan1taryComputer|ProcessInteraction(Message) (.hitcomponent _outhit))))

(event Input|EnhancedActionEvents|EnhancedInputActionIA_Move
  (params (ActionValue :type Vector%202D%20Structure) (ElapsedSeconds :type Float%20%28double-precision%29) (TriggeredSeconds :type Float%20%28double-precision%29) (InputAction :type Input%20Action%20Object%20Reference :default "/Game/EunrileneGene/Inputs/Action/IA_Move.IA_Move"))
  (bind _firstpersoncamera (Variables|MyCharacter|GetFirstPersonCamera))
  (bind _returnvalue (Transformation|GetWorldRotation _firstpersoncamera))
  ;[0.006671 0.151 0] Controls
  (:Triggered
    (Pawn|Input|AddMovementInput 0 (Math|Vector|GetForwardVector (Math|Rotator|MakeRotator 0.0 0.0 (.yaw _returnvalue))) (.x ActionValue) false)
    (Pawn|Input|AddMovementInput 0 (Math|Vector|GetRightVector (Math|Rotator|MakeRotator 0.0 0.0 (.yaw _returnvalue))) (.y ActionValue) false)))

(event EventPossessed
  (params (NewController :type Controller%20Object%20Reference))
  ;[1 0 0] Initializing Neural connections
  (bind _asplayer_controller (Utilities|Casting|CastToPlayerController NewController))
  (Input|AddMappingContext (PlayerController|LocalPlayerSubsystems|GetEnhancedInputLocalPlayerSubsystem _asplayer_controller) "/Game/EunrileneGene/Inputs/IMC_Movement.IMC_Movement" 0 "(bIgnoreAllPressedKeysUntilRelease=True,bForceImmediately=False,bNotifyUserSettings=False)"))

(event Collision|EventActorBeginOverlap
  (params (OtherActor :type Actor%20Object%20Reference))
  ;[1 0 0] ID
  (Class|BPIIdentity|CheckID(Message) OtherActor "id_29"))

(fn ConstructionScript
  (Utilities|FlowControl|Sequence
    (:then_0
      (AddComponent|AddAC0X00A21E))
    (:then_1)))